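; Anim notify state that ends a sandbox character's montage early while its window is active, based on a selectable blend-out condition.
; Each tick reads the owning pawn's animation properties through BPI_SandboxCharacter_Pawn and checks for forced blend-out, movement input, or falling.
; When the condition is met, it stops the montage with a configurable time and named blend profile, using a Hermite cubic blend.
; The notify's displayed name shows the selected condition.
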(fn ReceivedNotifyTick
  (params (MeshComp :type Skeletal%20Mesh%20Component%20Object%20Reference) (Animation :type Anim%20Sequence%20Base%20Object%20Reference) (FrameDeltaTime :type Float%20%28single-precision%29) (EventReference :type Anim%20Notify%20Event%20Reference%20Structure%20%28by%20ref%29))
  (bind _asbpi_sandbox_character_pawn (Utilities|Casting|CastToBPI_SandboxCharacter_Pawn (Components|GetOwner MeshComp)))
  (bind _returnvalue (Default|GetPropertiesforAnimation _asbpi_sandbox_character_pawn))
  (LocalVariables|SetCharacterProperties _returnvalue)
  (LocalVariables|SetAnimInstance (Components|SkeletalMesh|GetAnimInstance MeshComp))
  (bind _as动画蒙太奇 (Utilities|Casting|CastToAnimMontage Animation))
  (LocalVariables|SetAnimMontage _as动画蒙太奇)
  (Utilities|FlowControl|Sequence
    (:then_0
      (switch Utilities|FlowControl|Switch|SwitchonE_TraversalBlendOutCondition (Variables|Default|GetBlendOutCondition)
        (:NewEnumerator0
          (LocalVariables|SetShouldBlendOut true))
        (:NewEnumerator1
          (if (Utilities|Operators|NotEqual(!=) :A (.InputAcceleration (Utilities|Struct|BreakS_CharacterPropertiesForAnimation (LocalVariables|GetCharacterProperties))) :ErrorTolerance 0.1)
            (LocalVariables|SetShouldBlendOut true)))
        (:NewEnumerator2
          (if (Utilities|Enum|Equal(Enum) (.MovementMode (Utilities|Struct|BreakS_CharacterPropertiesForAnimation (LocalVariables|GetCharacterProperties))) "NewEnumerator5")
            (LocalVariables|SetShouldBlendOut true)))))
    (:then_1
      (if (LocalVariables|GetShouldBlendOut)
        (Class|AnimInstance|MontageStopwithBlendSettings (LocalVariables|GetAnimInstance) (Utilities|Struct|MakeMontageBlendSettings (Class|AnimInstance|GetBlendProfilebyName (LocalVariables|GetAnimInstance) (Variables|Default|GetBlendProfile)) (Utilities|Struct|MakeAlphaBlendArgs 0 (Variables|Default|GetBlendOutTime) "HermiteCubic") "Standard") (LocalVariables|GetAnimMontage))
        (return true)))))

(fn GetNotifyName
  (return (Utilities|String|Append "Early Blend out - " (Utilities|String|EnumtoString (Variables|Default|GetBlendOutCondition)))))