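; Anim notify state that overrides the collision response of the animated mesh owner's root component, presumably a character capsule, during an animation window.
; On begin it casts the root to a primitive component and sets the configurable NewResponse on all channels.
; On end, if ResetOnEnd is set, it applies the hard-coded CharacterCapsule profile with overlap updates, rather than restoring the previous responses.
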(fn ReceivedNotifyBegin
  (params (MeshComp :type Skeletal%20Mesh%20Component%20Object%20Reference) (Animation :type Anim%20Sequence%20Base%20Object%20Reference) (TotalDuration :type Float%20%28single-precision%29) (EventReference :type Anim%20Notify%20Event%20Reference%20Structure%20%28by%20ref%29))
  (bind _as基元组件 (Utilities|Casting|CastToPrimitiveComponent (Variables|/Script/Engine.Actor|GetRootComponent (Components|GetOwner MeshComp))))
  (Collision|SetCollisionResponsetoAllChannels _as基元组件 (Variables|Default|GetNew%20Response))
  (return false))

(fn ReceivedNotifyEnd
  (params (MeshComp :type Skeletal%20Mesh%20Component%20Object%20Reference) (Animation :type Anim%20Sequence%20Base%20Object%20Reference) (EventReference :type Anim%20Notify%20Event%20Reference%20Structure%20%28by%20ref%29))
  (if (Variables|Default|GetResetOnEnd)
    (bind _as基元组件 (Utilities|Casting|CastToPrimitiveComponent (Variables|/Script/Engine.Actor|GetRootComponent (Components|GetOwner MeshComp))))
    (Collision|SetCollisionProfileName _as基元组件 "CharacterCapsule" true :!class /Script/Engine.PrimitiveComponent)
    (return false)))