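; Anim notify that plays Minecraft (MC) footstep sounds matched to the surface under a character near the player.
; A downward complex sphere trace looks up the sound by physical material name prefix, then by the static mesh material at the hit face, falling back to Stone.
; The AC_FoleyEvents and default bank path is left unreachable, so the Event tag only labels the notify.
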(fn ReceivedNotify
  (params (MeshComp :type Skeletal%20Mesh%20Component%20Object%20Reference) (Animation :type Anim%20Sequence%20Base%20Object%20Reference) (EventReference :type Anim%20Notify%20Event%20Reference%20Structure%20%28by%20ref%29))
  (bind _returnvalue (Transformation|GetWorldLocation MeshComp))
  (bind (_outhit _returnvalue_2) (Collision|SphereTraceByChannel _returnvalue (- _returnvalue "0.000000,0.000000,50.000000") 25.0 "TraceTypeQuery1" true 0 "None" true "(R=1.000000,G=0.000000,B=0.000000,A=1.000000)" "(R=0.000000,G=1.000000,B=0.000000,A=1.000000)" 1.0))
  (if (and (< (Math|Vector|Distance(Vector) (Transformation|GetActorLocation (Game|Player|GetPlayerPawn 0)) _returnvalue) 7.5e+02) _returnvalue_2)
    (if (.ReturnValue (Utilities|Map|Find (Variables|Default|GetMC脚步声音效) (.LeftS (Utilities|String|Split (Utilities|GetDisplayName (.physmat _outhit)) "_"))))
      (LocalVariables|Set音效 (.Value (Utilities|Map|Find (Variables|Default|GetMC脚步声音效) (.LeftS (Utilities|String|Split (Utilities|GetDisplayName (.physmat _outhit)) "_")))))
      (else
        (Utilities|Casting|CastToStaticMeshComponent (.hitcomponent _outhit)
          (:then
            (bind (_成功 _匹配项) (CallFunction|映射字符串到音效 (Utilities|GetDisplayName (.ReturnValue (Class|PrimitiveComponent|GetMaterialfromCollisionFaceIndex (.hitcomponent _outhit) (.faceindex _outhit)))) (Variables|Default|GetMC脚步声音效)))
            (if _成功
              (LocalVariables|Set音效 _匹配项)
              (else
                (LocalVariables|Set音效 "/Game/Mineprep/音效/stone/stone.stone" :!label _label))))
          (:CastFailed
            (goto _label)))))
    (LocalVariables|SetMeshComponent MeshComp)
    (Audio|PlaySoundatLocation (LocalVariables|Get音效) (Transformation|GetWorldLocation (LocalVariables|GetMeshComponent)) "0, 0, 0" (Variables|Default|GetVolumeMultiplier) (Variables|Default|GetPitchMultiplier) 0.0 0 0 0 0)
    (return true)
    (else
      (return false))))

(fn GetNotifyName
  (return (Utilities|String|ToString(Text) (Utilities|Text|FormatText "FoleyEvent: {Type}" (.RightS (Utilities|String|Split (GameplayTags|GetDebugStringfromGameplayTag (Variables|Default|GetEvent)) "." "IgnoreCase" "FromEnd"))))))