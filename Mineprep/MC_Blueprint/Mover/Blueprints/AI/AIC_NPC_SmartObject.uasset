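; AI controller for NPCs, named for Smart Object use, that runs its behavior through a StateTree AI component.
; On BeginPlay it waits a second, then starts the StateTree logic manually.
; A Debug function draws a visual logger arrow from the controlled pawn along its control rotation to show facing.
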(event EventBeginPlay
  (Utilities|FlowControl|Delay 1.0)
  (AI|Logic|StartLogic (Variables|Default|GetStateTreeAI)))

(fn ConstructionScript)

(fn Debug
  (bind _returnvalue (Pawn|GetControlledPawn))
  (bind _returnvalue_2 (Transformation|GetActorLocation _returnvalue))
  (Class|DrawDebugLibrary|DrawDebugArrow (Class|DrawDebugLibrary|MakeVisualLoggerDebugDrawer "Draw Debug Library" "Display" true true) _returnvalue_2 (+ _returnvalue_2 (* (Math|Vector|GetForwardVector (Pawn|GetControlRotation _returnvalue :!class /Script/Engine.Pawn)) 5e+01)) "(Color=(R=1.000000,G=0.000000,B=1.000000,A=1.000000),Thickness=0.000000,LineType=Solid,DashWidth=2.500000,DashSpacing=1.000000,DotSpacing=1.000000)" true "(bArrowheadOnStart=False,bArrowLineEndsAtStartHead=False,ArrowHeadStartSize=5.000000,ArrowHeadStartType=Simple,bArrowheadOnEnd=True,bArrowLineEndsAtEndHead=False,ArrowHeadEndSize=5.000000,ArrowHeadEndType=Simple)"))