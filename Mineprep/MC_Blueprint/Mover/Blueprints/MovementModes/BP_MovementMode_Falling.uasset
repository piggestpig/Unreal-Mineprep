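; Falling movement mode for the Mover plugin that customizes how the character turns while airborne.
; GenerateMove runs the parent's move, then overrides only the proposed angular velocity.
; It turns the synced orientation toward the default input's orientation intent, with yaw shifted by a rotation offset from custom inputs.
; The turn rate is capped, and the step uses world delta seconds rather than the supplied simulation TimeStep.
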(fn GenerateMove
  (params (SimContext :type Mover%20Sim%20Context%20Structure%20%28by%20ref%29) (StartState :type Mover%20Tick%20Start%20Data%20Structure%20%28by%20ref%29) (TimeStep :type Mover%20Time%20Step%20Structure%20%28by%20ref%29) (OutProposedMove :type Proposed%20Move%20Structure%20%28by%20ref%29))
  (Utilities|FlowControl|Sequence
    (:then_0
      (LocalVariables|SetInputCollection (Utilities|Struct|BreakMoverInputCmdContext (Utilities|Struct|BreakMoverTickStartData StartState)))
      (bind _targetasrawbytes (Class|MoverDataCollectionLibrary|GetDatafromCollection (LocalVariables|GetInputCollection)))
      (LocalVariables|SetMoverDefaultInputs _targetasrawbytes)
      (bind _targetasrawbytes_2 (Class|MoverDataCollectionLibrary|GetDatafromCollection (LocalVariables|GetInputCollection)))
      (LocalVariables|SetMoverCustomInputs _targetasrawbytes_2))
    (:then_1
      (bind _targetasrawbytes_3 (Class|MoverDataCollectionLibrary|GetDatafromCollection (Utilities|Struct|BreakMoverSyncState (Utilities|Struct|BreakMoverTickStartData StartState))))
      (LocalVariables|SetSyncState _targetasrawbytes_3))
    (:then_2
      (|CallParentFunction SimContext StartState TimeStep OutProposedMove)
      (bind _returnvalue (Class|MovementUtils|ComputeAngularVelocityDegrees (Utilities|Struct|BreakMoverDefaultSyncState (LocalVariables|GetSyncState)) (Math|Rotator|MakeRotator (.roll (Math|Conversions|RotationFromXVector (Utilities|Struct|BreakCharacterDefaultInputs (LocalVariables|GetMoverDefaultInputs)))) (.pitch (Math|Conversions|RotationFromXVector (Utilities|Struct|BreakCharacterDefaultInputs (LocalVariables|GetMoverDefaultInputs)))) (+ (.yaw (Math|Conversions|RotationFromXVector (Utilities|Struct|BreakCharacterDefaultInputs (LocalVariables|GetMoverDefaultInputs)))) (Utilities|Struct|BreakS_MoverCustomInputs (LocalVariables|GetMoverCustomInputs)))) (Utilities|Time|GetWorldDeltaSeconds) 3e+02))
      (Utilities|Struct|SetmembersinProposedMove OutProposedMove _returnvalue)
      (return))))